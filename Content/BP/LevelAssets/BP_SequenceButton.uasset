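; BP_SequenceButton is a shootable target button for a sequence driven by a Manager, starting hidden with collision disabled.
; Activate reveals it with a red material and enables collision.
; The first hit from a BP_FirstPersonProjectile turns it green, spawns timed sparks, plays a sound at world origin, notifies the Manager and hides it again.
; IsActivated is never reset here, so each button registers only one shot.
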(event Custom|Activate
  (Rendering|Material|SetMaterial (Variables|Default|GetCylinder) 0 (Variables|Default|GetRedMaterial))
  (Rendering|SetActorHiddenInGame false)
  (Collision|SetActorEnableCollision true))

(event Custom|DeActivate
  (Rendering|SetActorHiddenInGame true)
  (Collision|SetActorEnableCollision false))

(event EventBeginPlay
  (Rendering|SetActorHiddenInGame true)
  (Collision|SetActorEnableCollision false))

(event Collision|EventHit
  (params (MyComp :type Primitive%20Component%20Object%20Reference) (Other :type Actor%20Object%20Reference) (OtherComp :type Primitive%20Component%20Object%20Reference) (bSelfMoved :type Boolean) (HitLocation :type Vector :default "0, 0, 0") (HitNormal :type Vector :default "0, 0, 0") (NormalImpulse :type Vector :default "0, 0, 0") (Hit :type Hit%20Result%20Structure%20%28by%20ref%29))
  (Utilities|Casting|CastToBP_FirstPersonProjectile Other)
  (if (not (Variables|Default|GetIsActivated))
    (Variables|Default|SetIsActivated true)
    (Rendering|Material|SetMaterial (Variables|Default|GetCylinder) 0 (Variables|Default|GetGreenMaterial))
    (bind _returnvalue (Game|SpawnActorfromClass "/Game/StarterContent/Blueprints/Blueprint_Effect_Sparks.Blueprint_Effect_Sparks_C" (Math|Transform|MakeTransform (Transformation|GetActorLocation) "90.000000,0.000000,0.000000") "Undefined" "MultiplyWithRoot" 0 0))
    (Actor|SetLifeSpan _returnvalue (Variables|Default|GetIn%20Lifespan))
    (Audio|PlaySoundatLocation "/Engine/VREditor/Sounds/UI/Dockable_Window_Drop.Dockable_Window_Drop" "0, 0, 0" "0, 0, 0" 1.0 1.0 0.0 0 0 0 0)
    (Default|ButtonShot (Variables|Default|GetManager))
    (CallFunction|DeActivate)))

(fn ConstructionScript)