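; BP_Checkpoint is a level checkpoint meant to record a respawn point and save state when its collision is overlapped.
; On first activation it writes its location to BP_FirstPersonGameMode, then calls SaveStateMessage on every BPI_Checkpoitable actor, playing a click sound for each.
; Both the character and game mode casts take the overlapping actor, so the chain stops before activation as wired.
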(event OnComponentBeginOverlap(Collision)
  (params (OverlappedComponent :type Primitive%20Component%20Object%20Reference) (OtherActor :type Actor%20Object%20Reference) (OtherComp :type Primitive%20Component%20Object%20Reference) (OtherBodyIndex :type Integer) (bFromSweep :type Boolean) (SweepResult :type Hit%20Result%20Structure%20%28by%20ref%29))
  (if (Variables|Default|GetActivated)
    (Development|PrintString "CheckPoint Already Active")
    (else
      (Development|PrintString "Checkpoint Activated")
      (Utilities|Casting|CastToBP_FirstPersonCharacter OtherActor)
      (bind _asbp_first_person_game_mode (Utilities|Casting|CastToBP_FirstPersonGameMode OtherActor))
      (Variables|Default|SetActivated true)
      (Variables|/Game/FirstPerson/Blueprints/BP_FirstPersonGameMode.BP_FirstPersonGameMode_C|SetLastcheckpointLocation _asbp_first_person_game_mode (Transformation|GetActorLocation))
      (Variables|/Game/FirstPerson/Blueprints/BP_FirstPersonGameMode.BP_FirstPersonGameMode_C|SetHasCheckpoint _asbp_first_person_game_mode true)
      (bind _outactors (Actor|GetAllActorswithInterface "/Game/BP/LogicBP/Visuals/BPI_Checkpoitable.BPI_Checkpoitable_C"))
      (for _array_element _outactors
        (Class|BPICheckpoitable|SaveState(Message) _array_element)
        (Audio|PlaySoundatLocation "/Engine/VREditor/Sounds/UI/Click_on_Button_Cue.Click_on_Button_Cue" "0, 0, 0" "0, 0, 0" 1.0 1.0 0.0 0 0 0 0)))))

(event EventBeginPlay)

(event Collision|EventActorBeginOverlap
  (params (OtherActor :type Actor%20Object%20Reference)))

(event EventTick
  (params (DeltaSeconds :type Float%20%28single-precision%29)))

(fn ConstructionScript)