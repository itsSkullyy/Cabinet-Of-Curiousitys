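; Manager for shootable buttons that opens a referenced door once enough buttons are activated.
; Each ButtonActivated call increments a counter until it reaches the required count.
; A one-shot flag then latches, a success sound plays at the world origin, and the door reference is cast to MoveBP to call DoorOpen.
; The manager only counts calls and does not track which button sent them.
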(event Custom|ButtonActivated
  (Development|PrintString "ButtonActivated")
  (if (not (Variables|Default|GetAlready%20Triggered))
    (bind _result (Math|Integer|IncrementInt (Variables|Default|GetActivatedCount))
      (:%20%20
        (Variables|Default|SetActivatedCount _result)
        (if (>= (Variables|Default|GetActivatedCount) (Variables|Default|GetRequiredCount))
          (Variables|Default|SetAlready%20Triggered true)
          (Audio|PlaySoundatLocation "/Engine/EditorSounds/Notifications/CompileSuccess.CompileSuccess" "0, 0, 0" "0, 0, 0" 1.0 1.0 0.0 0 0 0 0)
          (bind _asmove_bp (Utilities|Casting|CastToMoveBP (Variables|Default|GetDoorReference)))
          (Default|DoorOpen _asmove_bp))))))

(fn ConstructionScript)