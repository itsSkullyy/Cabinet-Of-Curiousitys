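; BP_ShootableButton is a level button that activates once when hit by a first-person projectile.
; It starts with a red material on its cylinder and turns green on the first valid hit, guarded by IsActivated.
; That hit also plays a ping at the world origin, notifies its Manager through ButtonActivated and destroys the projectile.
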(event EventBeginPlay
  (Rendering|Material|SetMaterial (Variables|Default|GetCylinder) 0 (Variables|Default|GetRedMaterial)))

(event Collision|EventHit
  (params (MyComp :type Primitive%20Component%20Object%20Reference) (Other :type Actor%20Object%20Reference) (OtherComp :type Primitive%20Component%20Object%20Reference) (bSelfMoved :type Boolean) (HitLocation :type Vector :default "0, 0, 0") (HitNormal :type Vector :default "0, 0, 0") (NormalImpulse :type Vector :default "0, 0, 0") (Hit :type Hit%20Result%20Structure%20%28by%20ref%29))
  (Utilities|Casting|CastToBP_FirstPersonProjectile Other)
  (if (not (Variables|Default|GetIsActivated))
    (Variables|Default|SetIsActivated true)
    (Rendering|Material|SetMaterial (Variables|Default|GetCylinder) 0 (Variables|Default|GetGreenMaterial))
    (Audio|PlaySoundatLocation "/Engine/EngineSounds/1kSineTonePing.1kSineTonePing" "0, 0, 0" "0, 0, 0" 1.0 1.0 0.0 0 0 0 0)
    (Default|ButtonActivated (Variables|Default|GetManager))
    (Actor|DestroyActor Other)))

(fn ConstructionScript)