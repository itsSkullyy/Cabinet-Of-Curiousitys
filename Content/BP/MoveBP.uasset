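; Moving door Blueprint that opens once its button-press count reaches three, printing progress messages on each press.
; Opening swaps to the Moving material, plays a metal door sound and starts a Timeline, whose position Tick applies while ShouldMove is set.
; The Timeline's finish clears the flag and restores the Idle material.
; DoorMove is a stub, and SetRandomDestination computes a random destination that the movement shown never reads.
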(event Custom|Door%20Open
  (Variables|Default|SetbShouldMove true)
  (Rendering|Material|SetMaterial (Variables|Default|GetStaticMesh) 0 "/Game/Materials/Moving.Moving")
  (Audio|PlaySoundatLocation "/Game/SFX/Metal_Door.Metal_Door" (stale _pos) "0, 0, 0" 1.0 1.0 0.0 0 0 0 0)
  (bind _pos (Timeline|Timeline PlayFromStart)
    (:Finished
      (Variables|Default|SetbShouldMove false)
      (Rendering|Material|SetMaterial (Variables|Default|GetStaticMesh) 0 "/Game/Materials/Idle.Idle"))))

(event EventBeginPlay
  (Variables|Default|SetbShouldMove false))

(event EventTick
  (params (DeltaSeconds :type Float%20%28single-precision%29))
  (if (Variables|Default|GetbShouldMove)
    (Transformation|SetActorLocation (stale _pos) false false)
    (else
      (bind _pos (Timeline|Timeline Stop)
        (:Finished
          (Variables|Default|SetbShouldMove false)
          (Rendering|Material|SetMaterial (Variables|Default|GetStaticMesh) 0 "/Game/Materials/Idle.Idle"))))))

(fn ConstructionScript)

(fn DoorOpen
  (Variables|Default|SetButtonsPressed (+ (Variables|Default|GetButtonsPressed) 1))
  (if (>= (Variables|Default|GetButtonsPressed) 3)
    (Development|PrintString "Access Granted")
    (CallFunction|DoorOpen)
    (else
      (Development|PrintString "Button Pressed"))))